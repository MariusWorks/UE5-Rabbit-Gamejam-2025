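; Pooled melee enemy that chases the player and attacks in close range, using stats from EnemyStats.
; Tick drives movement, cooldown and a curve-tilted windup, ending in a forward trace that deals damage or triggers the player's shield block.
; Hits cause timeline knockback; lethal ones play a knock-away, sink and tip-over, then notify BP_EnemyManager.
; Enable and Disable toggle tick, collision and visibility, parking inactive enemies below the world.
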(event EventBeginPlay
  (Utilities|IsValid (Variables|Default|GetManagerRef)
    (:Is%20Valid
      _)
    (:Is%20Not%20Valid
      (bind _returnvalue (Actor|GetActorOfClass "/Game/Blueprints/Enemy/BP_EnemyManager.BP_EnemyManager_C"))
      (Variables|Default|SetManagerRef _returnvalue)))
  (Utilities|IsValid (Variables|Default|GetPlayerRef)
    (:Is%20Not%20Valid
      (Variables|Default|SetPlayerRef (Game|Player|GetPlayerPawn 0)))))

(event EventTick
  (params (DeltaSeconds :type Float%20%28single-precision%29))
  (CallFunction|MoveTowardsPlayer)
  (CallFunction|RechargeAttack)
  (if (and (Variables|Default|GetbInCombatRange) (<= (Variables|Timers|GetEnemyAttackCooldown) 0.0))
    (CallFunction|WindupAttack)
    (if (>= (Variables|Timers|GetEnemyAttackWindupTimer) (.AttackDuration (Utilities|Struct|BreakS_EnemyStats (Variables|Default|GetEnemyStats))))
      (Transformation|SetRelativeRotation (Variables|Default|GetCube) (Math|Rotator|MakeRotator 0.0 0.0 0.0) false false)
      (Variables|Timers|SetEnemyAttackWindupTimer 0.0)
      (Variables|Timers|SetEnemyAttackCooldown (.AattackCooldown (Utilities|Struct|BreakS_EnemyStats (Variables|Default|GetEnemyStats))))
      (CallFunction|AttackPlayer))))

(event EventOnDamage
  (params (Damage :type Float%20%28double-precision%29) (Attacker :type Actor%20Object%20Reference))
  (bind _returnvalue (Transformation|GetActorLocation))
  (bind _enemystats (Variables|Default|GetEnemyStats))
  (bind _health (Utilities|Struct|BreakS_EnemyStats _enemystats))
  (bind _returnvalue_2 (- _health Damage))
  (bind _returnvalue_3 (<= _returnvalue_2 0.0))
  (Development|PrintString (Utilities|String|ToString(Text) (Utilities|Text|FormatText "{Attacker} Dealt {Damage} Damage to {ThisActor}" (Utilities|GetDisplayName Attacker) Damage (Utilities|GetDisplayName self))) false)
  (|SetBy-RefVar _health (select _returnvalue_3 0.0 _returnvalue_2))
  (Variables|Default|SetKnockbackDirection (Math|Vector2D|Normalize2D (- (Math|Conversions|ToVector2D(Vector) (Transformation|GetActorLocation)) (Math|Conversions|ToVector2D(Vector) (Transformation|GetActorLocation Attacker)))))
  (if _returnvalue_3
    (Class|BPIPlayerState|AddKill(Message) (Game|GetPlayerController 0) (Utilities|Struct|BreakS_EnemyStats (Variables|Default|GetEnemyStats)))
    (Variables|Default|SetDeathStartLocation _returnvalue)
    (Variables|Default|SetDeathEndLocation (+ _returnvalue (* 5e+02 (Variables|Default|GetKnockbackDirection))))
    (Collision|SetCollisionEnabled (Variables|Default|GetBox) "NoCollision")
    (bind (_direction _knockback_alpha _rotation_alpha _sink_alpha) (Timeline|Timeline_Death PlayFromStart)
      (:Update
        (Transformation|SetActorLocation (Math|Interpolation|Ease "EaseOut" _knockback_alpha (Variables|Default|GetDeathStartLocation) (Math|Vector|MakeVector (.X (Math|Vector|BreakVector (Variables|Default|GetDeathEndLocation))) (.Y (Math|Vector|BreakVector (Variables|Default|GetDeathEndLocation))) (Math|Float|Lerp (.Z (Math|Vector|BreakVector (Variables|Default|GetDeathEndLocation))) (- (.Z (Math|Vector|BreakVector (Variables|Default|GetDeathEndLocation))) 2e+02) _sink_alpha)) 2.0) false false)
        (Transformation|SetRelativeRotation (Variables|Default|GetCube) (Math|Interpolation|Ease :Function "EaseOut" :Alpha _rotation_alpha :B "90.000000,0.000000,0.000000" :ShortestPath false) false false))
      (:Finished
        (Default|HandleEnemyDeath (Variables|Default|GetManagerRef) self)))
    (else
      (Timeline|Timeline_Knockback PlayFromStart
        (:Update
          (Transformation|AddActorWorldOffset (* (Variables|Default|GetKnockbackDirection) (* 5e+02 (Utilities|Time|GetWorldDeltaSeconds))) true))))))

(event EventDisable
  (Actor|Tick|SetActorTickEnabled false)
  (Variables|/Script/Engine.PrimitiveComponent|SetbGenerateOverlapEvents (Variables|Default|GetBox) false)
  (Collision|SetCollisionEnabled (Variables|Default|GetBox) "NoCollision")
  (Rendering|SetActorHiddenInGame true)
  (Transformation|SetActorLocationAndRotation "0.000000,0.000000,-5000.000000" "0, 0, 0" false true))

(event EventEnable
  (params (SpawnLocation :type Vector :default "0, 0, 0"))
  (Actor|Tick|SetActorTickEnabled true)
  (Variables|/Script/Engine.PrimitiveComponent|SetbGenerateOverlapEvents (Variables|Default|GetBox) true)
  (Collision|SetCollisionEnabled (Variables|Default|GetBox) "QueryAndPhysics")
  (Rendering|SetActorHiddenInGame false)
  (Transformation|SetActorLocationAndRotation SpawnLocation "0, 0, 0" false true))

(fn ConstructionScript)

(fn MoveTowardsPlayer
  (LocalVariables|Set_PlayerLocation (Math|Conversions|ToVector2D(Vector) (Transformation|GetActorLocation (Variables|Default|GetPlayerRef))))
  (LocalVariables|Set_ActorLocation (Math|Conversions|ToVector2D(Vector) (Transformation|GetActorLocation)))
  (if (< (Math|Vector2D|Vector2DLength (- (LocalVariables|Get_PlayerLocation) (LocalVariables|Get_ActorLocation))) 175.0)
    (Variables|Default|SetbInCombatRange true)
    (else
      (Variables|Default|SetbInCombatRange false)))
  (if (< (Math|Vector2D|Vector2DLength (- (LocalVariables|Get_PlayerLocation) (LocalVariables|Get_ActorLocation))) 1.5e+02)
    _
    (else
      (Transformation|AddActorWorldOffset (Math|Conversions|ToVector(Vector2D) (* (Math|Vector2D|Normalize2D (- (LocalVariables|Get_PlayerLocation) (LocalVariables|Get_ActorLocation))) (* (Utilities|Time|GetWorldDeltaSeconds) (.Speed (Utilities|Struct|BreakS_EnemyStats (Variables|Default|GetEnemyStats)))))) true)))
  (Transformation|SetActorRotation (Math|Rotator|FindLookatRotation (Math|Conversions|ToVector(Vector2D) (LocalVariables|Get_ActorLocation)) (Math|Conversions|ToVector(Vector2D) (LocalVariables|Get_PlayerLocation)))))

(fn AttackPlayer
  (bind _returnvalue (Transformation|GetActorLocation))
  (bind (_outhit _returnvalue_2) (Collision|LineTraceForObjects _returnvalue (+ _returnvalue (* (Transformation|GetActorForwardVector) 1.5e+02)) (Utilities|Array|MakeArray "ObjectTypeQuery3") false (Utilities|Array|MakeArray self) "None"))
  (if (and _returnvalue_2 (Utilities|DoesObjectImplementInterface (.HitActor (Collision|BreakHitResult _outhit)) "/Game/Blueprints/Player/BPI_Player.BPI_Player_C"))
    (if (== (Utilities|GetClass (.HitComponent (Collision|BreakHitResult _outhit))) "/Script/Engine.CapsuleComponent")
      (Class|BPICombat|OnDamage(Message) (.HitActor (Collision|BreakHitResult _outhit)) (.Damage (Utilities|Struct|BreakS_EnemyStats (Variables|Default|GetEnemyStats))) self :!label _label)
      (elif (== (Utilities|GetClass (.HitComponent (Collision|BreakHitResult _outhit))) "/Script/Engine.BoxComponent")
        (bind _bcanblock (Class|BPICombat|GetCanBlock(Message) (.HitActor (Collision|BreakHitResult _outhit))))
        (if _bcanblock
          (Class|BPICombat|OnShield(Message) (.HitActor (Collision|BreakHitResult _outhit)))
          (else
            (goto _label)))))))

(fn RechargeAttack
  (Variables|Timers|SetEnemyAttackCooldown (select (<= (- (Variables|Timers|GetEnemyAttackCooldown) (Utilities|Time|GetWorldDeltaSeconds)) 0.0) 0.0 (- (Variables|Timers|GetEnemyAttackCooldown) (Utilities|Time|GetWorldDeltaSeconds)))))

(fn WindupAttack
  (bind _output_get (Variables|Timers|SetEnemyAttackWindupTimer (Math|Float|Clamp(Float) (+ (Variables|Timers|GetEnemyAttackWindupTimer) (Utilities|Time|GetWorldDeltaSeconds)) 0.0 (.AttackDuration (Utilities|Struct|BreakS_EnemyStats (Variables|Default|GetEnemyStats))))))
  (Transformation|SetRelativeRotation (Variables|Default|GetCube) (Math|Rotator|MakeRotator 0.0 (* (Math|Curves|GetFloatValue (Variables|Default|GetAttackCurve) (/ _output_get (.AttackDuration (Utilities|Struct|BreakS_EnemyStats (Variables|Default|GetEnemyStats))))) 2e+01) 0.0) false false))

(fn GetCanBlock
  (return false))