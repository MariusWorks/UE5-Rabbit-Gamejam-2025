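; Enemy manager that spawns pooled BP_Enemy actors on a randomized timer while the game runs, faster at night.
; Picks a random point in one of four edge boxes, skipping boxes overlapped by interface-implementing actors.
; Rolls a tier from day or night weights, then configures the enemy with that tier's mesh, extent and data table stats.
; Deaths return enemies to the pool; day begin kills tracked NightElites, which are top-tier enemies recorded during day spawns.
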(event OnComponentBeginOverlap(TopBoxRef)
  (params (OverlappedComponent :type Primitive%20Component%20Object%20Reference) (OtherActor :type Actor%20Object%20Reference) (OtherComp :type Primitive%20Component%20Object%20Reference) (OtherBodyIndex :type Integer) (bFromSweep :type Boolean) (SweepResult :type Hit%20Result%20Structure%20%28by%20ref%29))
  (CallFunction|UpdateBox OtherActor false (Variables|Default|GetTopBoxRef)))

(event OnComponentEndOverlap(TopBoxRef)
  (params (OverlappedComponent :type Primitive%20Component%20Object%20Reference) (OtherActor :type Actor%20Object%20Reference) (OtherComp :type Primitive%20Component%20Object%20Reference) (OtherBodyIndex :type Integer))
  (CallFunction|UpdateBox OtherActor true (Variables|Default|GetTopBoxRef)))

(event OnComponentBeginOverlap(LeftBoxRef)
  (params (OverlappedComponent :type Primitive%20Component%20Object%20Reference) (OtherActor :type Actor%20Object%20Reference) (OtherComp :type Primitive%20Component%20Object%20Reference) (OtherBodyIndex :type Integer) (bFromSweep :type Boolean) (SweepResult :type Hit%20Result%20Structure%20%28by%20ref%29))
  (CallFunction|UpdateBox OtherActor false (Variables|Default|GetLeftBoxRef)))

(event OnComponentEndOverlap(LeftBoxRef)
  (params (OverlappedComponent :type Primitive%20Component%20Object%20Reference) (OtherActor :type Actor%20Object%20Reference) (OtherComp :type Primitive%20Component%20Object%20Reference) (OtherBodyIndex :type Integer))
  (CallFunction|UpdateBox OtherActor true (Variables|Default|GetLeftBoxRef)))

(event OnComponentBeginOverlap(BottomBoxRef)
  (params (OverlappedComponent :type Primitive%20Component%20Object%20Reference) (OtherActor :type Actor%20Object%20Reference) (OtherComp :type Primitive%20Component%20Object%20Reference) (OtherBodyIndex :type Integer) (bFromSweep :type Boolean) (SweepResult :type Hit%20Result%20Structure%20%28by%20ref%29))
  (CallFunction|UpdateBox OtherActor false (Variables|Default|GetBottomBoxRef)))

(event OnComponentEndOverlap(BottomBoxRef)
  (params (OverlappedComponent :type Primitive%20Component%20Object%20Reference) (OtherActor :type Actor%20Object%20Reference) (OtherComp :type Primitive%20Component%20Object%20Reference) (OtherBodyIndex :type Integer))
  (CallFunction|UpdateBox OtherActor true (Variables|Default|GetBottomBoxRef)))

(event OnComponentBeginOverlap(RightBoxRef)
  (params (OverlappedComponent :type Primitive%20Component%20Object%20Reference) (OtherActor :type Actor%20Object%20Reference) (OtherComp :type Primitive%20Component%20Object%20Reference) (OtherBodyIndex :type Integer) (bFromSweep :type Boolean) (SweepResult :type Hit%20Result%20Structure%20%28by%20ref%29))
  (CallFunction|UpdateBox OtherActor false (Variables|Default|GetRightBoxRef)))

(event OnComponentEndOverlap(RightBoxRef)
  (params (OverlappedComponent :type Primitive%20Component%20Object%20Reference) (OtherActor :type Actor%20Object%20Reference) (OtherComp :type Primitive%20Component%20Object%20Reference) (OtherBodyIndex :type Integer))
  (CallFunction|UpdateBox OtherActor true (Variables|Default|GetRightBoxRef)))

(event Custom|OnDayBegin
  (Variables|Default|SetbIsDay true)
  (CallFunction|CullNightElites))

(event Custom|OnNightBegin
  (Variables|Default|SetbIsDay false))

(event Custom|OnGameBegin
  (Actor|Tick|SetActorTickEnabled true))

(event Custom|OnGameEnd
  (Actor|Tick|SetActorTickEnabled false))

(event EventBeginPlay
  (bind _gamestate (Class|BPIGameState|GetInstance(Message) (Game|GetGameState)))
  (EventDispatchers|BindEventtoOnGameBeginDispatcher _gamestate (EventDispatchers|CreateEvent :!event Custom|OnGameBegin))
  (EventDispatchers|BindEventtoOnGameEndDispatcher _gamestate (EventDispatchers|CreateEvent :!event Custom|OnGameEnd))
  (EventDispatchers|BindEventtoOnDayBeginDispatcher _gamestate (EventDispatchers|CreateEvent :!event Custom|OnDayBegin))
  (EventDispatchers|BindEventtoOnNightBeginDispatcher _gamestate (EventDispatchers|CreateEvent :!event Custom|OnNightBegin))
  (bind _outactors (Actor|GetAllActorsOfClass "/Game/Blueprints/Enemy/BP_Enemy.BP_Enemy_C"))
  (for _array_element _outactors
    (Utilities|Map|Add (Variables|Default|GetEnemyPool) _array_element true))
  (CallFunction|InitializeEnemyPool))

(event EventTick
  (params (DeltaSeconds :type Float%20%28single-precision%29))
  (bind _output_get (Variables|Default|SetSpawnTimer (+ DeltaSeconds (Variables|Default|GetSpawnTimer))))
  (if (> _output_get (select (Variables|Default|GetbIsDay) (Math|Random|RandomFloatinRange 1.0 1.3) (Math|Random|RandomFloatinRange 0.6 0.9)))
    (Variables|Default|SetSpawnTimer 0.0)
    (bind _spawnlocation (CallFunction|GetSpawnLocation))
    (bind _freeenemy (CallFunction|GetFreeEnemy))
    (Utilities|IsValid _freeenemy
      (:Is%20Valid
        (bind _enemytier (CallFunction|GetEnemyTier))
        (if (and (> _enemytier 3) (Variables|Default|GetbIsDay))
          (Utilities|Array|Add (Variables|Default|GetNightElites) _freeenemy))
        (bind (_boxextent _mesh _stats) (CallFunction|SetupEnemy _enemytier))
        (Class|BPIEnemy|Enable(Message) _freeenemy _spawnlocation _boxextent _mesh _stats)
        (Development|PrintString "New Enemy Spawned!" false))
      (:Is%20Not%20Valid
        (Development|PrintString "WARNING: No more enemies in pool!" false)))))

(fn ConstructionScript
  (bind _box (CallFunction|SetupBox (Variables|Positions|GetTopBoxPosition) (Variables|Scale|GetTopBoxScale)))
  (Variables|Default|SetTopBoxRef _box)
  (bind _box_2 (CallFunction|SetupBox (Variables|Positions|GetLeftBoxPosition) (Variables|Scale|GetLeftBoxScale)))
  (Variables|Default|SetLeftBoxRef _box_2)
  (bind _box_3 (CallFunction|SetupBox (Variables|Positions|GetBottomBoxPosition) (Variables|Scale|GetBottomBoxScale)))
  (Variables|Default|SetBottomBoxRef _box_3)
  (bind _box_4 (CallFunction|SetupBox (Variables|Positions|GetRightBoxPosition) (Variables|Scale|GetRightBoxScale)))
  (Variables|Default|SetRightBoxRef _box_4))

(fn InitializeEnemyPool
  (bind _returnvalue (Actor|GetActorOfClass "/Game/Blueprints/Player/BP_PlayerPawn.BP_PlayerPawn_C"))
  (LocalVariables|Set_PlayerRef _returnvalue)
  (for _index (range 1 (Variables|Default|GetEnemyPoolSize))
    (bind _returnvalue_2 (Game|SpawnActorfromClass "/Game/Blueprints/Enemy/BP_Enemy.BP_Enemy_C" (Math|Transform|MakeTransform "0.000000,0.000000,-500.000000") "AlwaysSpawn" "MultiplyWithRoot" 0 (LocalVariables|Get_PlayerRef) self 0))
    (Utilities|Map|Add (Variables|Default|GetEnemyPool) _returnvalue_2 false)))

(fn GetFreeEnemy
  (bind _keys (Utilities|Map|Keys (Variables|Default|GetEnemyPool)))
  (LocalVariables|Set_EnemyPoolKeys _keys)
  (bind _values (Utilities|Map|Values (Variables|Default|GetEnemyPool)))
  (if (!= (Utilities|Array|FindItem _values false) -1)
    (Utilities|Map|Add (Variables|Default|GetEnemyPool) (Utilities|Array|Get(acopy) (LocalVariables|Get_EnemyPoolKeys) (Utilities|Array|FindItem _values false)) true)
    (return (Utilities|Array|Get(acopy) (LocalVariables|Get_EnemyPoolKeys) (Utilities|Array|FindItem _values false)))
    (else
      (return 0))))

(fn SetupBox
  (params (Position :type Vector) (Scale :type Vector))
  (bind _returnvalue (AddComponent|AddBoxComponent false (Math|Transform|MakeTransform Position)))
  (Components|Box|SetBoxExtent _returnvalue Scale false)
  (Development|SetHiddeninGame _returnvalue true false)
  (Utilities|Map|Add (Variables|Default|GetBoxMap) _returnvalue true)
  (return _returnvalue))

(fn UpdateBox
  (params (OtherActor :type Object%20Object%20Reference) (bMarkAsAvailable :type Boolean) (Box :type Box%20Component%20Object%20Reference))
  (if (Utilities|DoesObjectImplementInterface OtherActor 0)
    (Utilities|Map|Add (Variables|Default|GetBoxMap) Box bMarkAsAvailable)))

(fn GetSpawnLocation
  (bind __availableboxspawns (LocalVariables|Get_AvailableBoxSpawns))
  (bind _outitem (Utilities|Array|Random __availableboxspawns))
  (bind _returnvalue (Transformation|GetWorldLocation _outitem))
  (bind _returnvalue_2 (Components|Box|GetScaledBoxExtent _outitem))
  (bind _returnvalue_3 (Math|Random|RandomPointinBoundingBox _returnvalue _returnvalue_2))
  (bind (_x _y) (Math|Vector|BreakVector _returnvalue_3))
  (bind _keys (Utilities|Map|Keys (Variables|Default|GetBoxMap)))
  (for _array_element _keys
    (if (.Value (Utilities|Map|Find (Variables|Default|GetBoxMap) _array_element))
      (Utilities|Array|Add (LocalVariables|Get_AvailableBoxSpawns) _array_element)))
  (if (Utilities|Array|IsEmpty (LocalVariables|Get_AvailableBoxSpawns))
    (return "0, 0, 0")
    (else
      (return (Math|Vector|MakeVector _x _y 5e+01)))))

(fn HandleEnemyDeath
  (params (Actor :type Actor%20Object%20Reference))
  (Utilities|Map|Add (Variables|Default|GetEnemyPool) Actor false)
  (Class|BPIEnemy|Disable(Message) Actor))

(fn PrintEnemyPool
  (LocalVariables|Set_PoolSize (Utilities|Map|Length (Variables|Default|GetEnemyPool)))
  (bind _values (Utilities|Map|Values (Variables|Default|GetEnemyPool)))
  (bind _keys (Utilities|Map|Keys (Variables|Default|GetEnemyPool)))
  (for (_ _array_index) _keys
    (if (Utilities|Array|Get(acopy) _values _array_index)
      (Math|Integer|IncrementInt (LocalVariables|Get_PoolUsed))
      (else
        (Math|Integer|IncrementInt (LocalVariables|Get_PoolFree)))))
  (Development|PrintString (Utilities|String|ToString(Text) (Utilities|Text|FormatText "Enemy Pool Size: {EnemyPoolSize} 
Free: {Free} 
Used: {Used}" (LocalVariables|Get_PoolSize) (LocalVariables|Get_PoolFree) (LocalVariables|Get_PoolUsed))) true false "(R=1.000000,G=0.000000,B=0.000000,A=1.000000)" 2.0 "Pool"))

(fn GetEnemyTier
  (LocalVariables|Set_RandomFloat (Math|Random|RandomFloatinRange 0.0 1e+02))
  (for (_array_element _array_index) (select (Variables|Default|GetbIsDay) (Variables|Default|GetEnemyDayWeights) (Variables|Default|GetEnemyNightWeights))
    (bind _output_get (LocalVariables|Set_CurrentThreshold (+ _array_element (LocalVariables|Get_CurrentThreshold))))
    (if (<= (LocalVariables|Get_RandomFloat) _output_get)
      (return _array_index))))

(fn SetupEnemy
  (params (EnemyTier :type Integer))
  (switch int EnemyTier
    (:0
      (bind _returnvalue (Utilities|GetDataTableRow (Variables|Default|GetEnemyTable) "Fly")
        (:then
          (return "50.000000,50.000000,50.000000" "/Game/StaticMesh/Enemy_Fly.Enemy_Fly" _returnvalue))
        (:RowNotFound
          (return "50.000000,50.000000,50.000000" "/Engine/BasicShapes/Cube.Cube" ""))))
    (:1
      (bind _returnvalue_2 (Utilities|GetDataTableRow (Variables|Default|GetEnemyTable) "Caterpillar")
        (:then
          (return "75.000000,50.000000,50.000000" "/Game/StaticMesh/Enemy_caterpillar.Enemy_caterpillar" _returnvalue_2))
        (:RowNotFound
          (return "50.000000,50.000000,50.000000" "/Engine/BasicShapes/Cube.Cube" ""))))
    (:2
      (bind _returnvalue_3 (Utilities|GetDataTableRow (Variables|Default|GetEnemyTable) "Beetle")
        (:then
          (return "60.000000,50.000000,50.000000" "/Game/StaticMesh/Enemy_Beetle.Enemy_Beetle" _returnvalue_3))
        (:RowNotFound
          (return "50.000000,50.000000,50.000000" "/Engine/BasicShapes/Cube.Cube" ""))))
    (:3
      (bind _returnvalue_4 (Utilities|GetDataTableRow (Variables|Default|GetEnemyTable) "Locust")
        (:then
          (return "60.000000,50.000000,50.000000" "/Game/StaticMesh/Enemy_Locust.Enemy_Locust" _returnvalue_4))
        (:RowNotFound
          (return "50.000000,50.000000,50.000000" "/Engine/BasicShapes/Cube.Cube" ""))))
    (:4
      (bind _returnvalue_5 (Utilities|GetDataTableRow (Variables|Default|GetEnemyTable) "Snail")
        (:then
          (return "80.000000,50.000000,50.000000" "/Game/StaticMesh/Enemy_snail.Enemy_snail" _returnvalue_5))
        (:RowNotFound
          (return "50.000000,50.000000,50.000000" "/Engine/BasicShapes/Cube.Cube" ""))))))

(fn CullNightElites
  (if (not (Utilities|Array|IsEmpty (Variables|Default|GetNightElites)))
    (for _array_element (Variables|Default|GetNightElites)
      (Class|BPIEnemy|Kill(Message) _array_element))
    (Utilities|Array|Clear (Variables|Default|GetNightElites))))