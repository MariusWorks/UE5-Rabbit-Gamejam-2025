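; Game state that runs the day/night cycle and handles game start, end and pause events.
; Tick advances a looping cycle timer, lerping the BP_Light sun's pitch (stored as Yaw) between sunrise and sunset angles and deriving its intensity from that angle.
; Paired DoOnce nodes reset each other so day and night dispatchers fire once per transition.
; Start and end toggle ticking, and DebugNight disables it at BeginPlay with a dark sun.
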(event Custom|OnDayBegin
  (Utilities|FlowControl|Sequence
    (:then_0
      (Utilities|FlowControl|DoOnce false
        (:Completed
          (Variables|Time|SetbIsNight false)
          (Default|CallOnDayBeginDispatcher))))
    (:then_1
      (Utilities|FlowControl|DoOnce false) ; enters at Reset
    )))

(event Custom|OnNightBegin
  (Utilities|FlowControl|Sequence
    (:then_0
      (Utilities|FlowControl|DoOnce false
        (:Completed
          (Variables|Time|SetbIsNight true)
          (Default|CallOnNightBeginDispatcher))))
    (:then_1
      (Utilities|FlowControl|DoOnce false) ; enters at Reset
    )))

(event Custom|OnGameEnd
  (Actor|Tick|SetActorTickEnabled false)
  (Variables|Default|SetbGameRunning false))

(event Custom|OnGameStart
  (Actor|Tick|SetActorTickEnabled true)
  (Variables|Default|SetbGameRunning true))

(event Custom|OnGamePaused
  (params (bGamePaused :type Boolean))
  (bind _output_get (Variables|Default|SetbGameIsPaused bGamePaused))
  (Game|SetGamePaused _output_get))

(event EventBeginPlay
  (EventDispatchers|BindEventtoOnGameBeginDispatcher (EventDispatchers|CreateEvent :!event Custom|OnGameStart))
  (EventDispatchers|BindEventtoOnGameEndDispatcher (EventDispatchers|CreateEvent :!event Custom|OnGameEnd))
  (EventDispatchers|BindEventtoOnGamePausedDispatcher (EventDispatchers|CreateEvent :!event Custom|OnGamePaused))
  (CallFunction|CalculateDayNightCycle)
  (bind _returnvalue (Actor|GetActorOfClass "/Game/Blueprints/Level/BP_Light.BP_Light_C"))
  (bind _output_get (Variables|Default|SetLightRef _returnvalue))
  (Transformation|SetActorRotation _output_get (Math|Rotator|MakeRotator 0.0 (Variables|Time|GetSunriseYaw) -9e+01))
  (if (Variables|Default|GetbDebugNight)
    (Actor|Tick|SetActorTickEnabled false)
    (Transformation|SetActorRotation (Variables|Default|GetLightRef) "-270.000000,-90.000000,0.000000")
    (Rendering|Components|Light|SetIntensity (Variables|/Game/Blueprints/Level/BP_Light.BP_Light_C|GetSun (Variables|Default|GetLightRef)) 0.0)))

(event EventTick
  (params (DeltaSeconds :type Float%20%28single-precision%29))
  (CallFunction|CalculateSun DeltaSeconds)
  (Transformation|SetActorRotation (Variables|Default|GetLightRef) (Math|Rotator|MakeRotator 0.0 (Variables|Time|GetYaw) -9e+01))
  (Rendering|Components|Light|SetIntensity (Variables|/Game/Blueprints/Level/BP_Light.BP_Light_C|GetSun (Variables|Default|GetLightRef)) (Variables|Time|GetCurrentIntensity))
  (if (> (Variables|Time|GetCycleTime) (Variables|Time|GetTotalLength))
    (Variables|Time|SetCycleTime 0.0)))

(fn ConstructionScript)

(fn CalculateDayNightCycle
  (Variables|Time|SetTotalLength (+ (Variables|Time|GetDayLength) (Variables|Time|GetNightLength)))
  (bind _output_get (Variables|Time|SetDaySpan (Math|Float|Absolute(Float) (- (Variables|Time|GetSunsetYaw) (Variables|Time|GetSunriseYaw)))))
  (Variables|Time|SetNightSpan (- 3.6e+02 _output_get)))

(fn CalculateSun
  (params (DeltaTime :type Float%20%28single-precision%29))
  (bind _output_get (Variables|Time|SetCycleTime (+ DeltaTime (Variables|Time|GetCycleTime))))
  (if (< _output_get (Variables|Time|GetDayLength))
    (Variables|Time|SetYaw (Math|Float|Lerp (Variables|Time|GetSunriseYaw) (Variables|Time|GetSunsetYaw) (/ (Variables|Time|GetCycleTime) (Variables|Time|GetDayLength))))
    (CallFunction|OnDayBegin)
    (else
      (Variables|Time|SetYaw (Math|Float|Lerp (Variables|Time|GetSunsetYaw) (- (Variables|Time|GetSunriseYaw) 3.6e+02) (/ (- (Variables|Time|GetCycleTime) (Variables|Time|GetDayLength)) (Variables|Time|GetNightLength))))
      (CallFunction|OnNightBegin)))
  (if (<= (Math|Float|Absolute(Float) (Variables|Time|GetYaw)) 1e+01)
    (Variables|Time|SetCurrentIntensity (Math|Float|Lerp (Variables|Time|GetNightIntensity) (Variables|Time|GetDayIntensity) (Math|Float|MapRangeClamped (Math|Float|Absolute(Float) (Variables|Time|GetYaw)) 0.0 1e+01 0.0 1.0)))
    (elif (<= (Math|Float|Absolute(Float) (Variables|Time|GetYaw)) 1.7e+02)
      (Variables|Time|SetCurrentIntensity (Variables|Time|GetDayIntensity))
      (elif (<= (Math|Float|Absolute(Float) (Variables|Time|GetYaw)) 1.8e+02)
        (Variables|Time|SetCurrentIntensity (Math|Float|Lerp (Variables|Time|GetDayIntensity) (Variables|Time|GetNightIntensity) (Math|Float|MapRangeClamped (Math|Float|Absolute(Float) (Variables|Time|GetYaw)) 1.7e+02 1.8e+02 0.0 1.0)))
        (elif (>= (Math|Float|Absolute(Float) (Variables|Time|GetYaw)) 1.8e+02)
          (Variables|Time|SetCurrentIntensity (Variables|Time|GetNightIntensity))
          (elif (>= (Math|Float|Absolute(Float) (Variables|Time|GetYaw)) 3.6e+02)
            (Variables|Time|SetCurrentIntensity (Math|Float|Lerp (Variables|Time|GetNightIntensity) (Variables|Time|GetDayIntensity) (Math|Float|MapRangeClamped (Math|Float|Absolute(Float) (Variables|Time|GetYaw)) 3.6e+02 3.7e+02 0.0 1.0)))))))))

(fn PrintDayInfo
  (Development|PrintString (Utilities|String|ToString(Text) (Utilities|Text|FormatText "Time: {Time} / {Length} 
Is Night: {IsNight} 
Sun Yaw: {SunYaw}" (Utilities|Text|ToText(Float) (Variables|Time|GetCycleTime) "HalfToEven" false true 1 324 1 1) (Variables|Time|GetTotalLength) (Variables|Time|GetbIsNight) (Variables|Time|GetYaw))) true false "(R=1.000000,G=0.849803,B=0.000000,A=1.000000)" 2.0 "Time"))

(fn GetInstance
  (return self))