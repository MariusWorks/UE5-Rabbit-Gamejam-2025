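; BP_Orb is a pooled energy pickup that homes in on the player and grants its OrbEnergy.
; A sphere overlap with a BPI_Player actor's sphere component stores the player and enables Tick, which interpolates the orb toward them.
; Within a short horizontal distance, it sends the energy message and returns itself to OrbManagerRef.
; Enable and Disable toggle visibility, collision and tick for reuse, with Enable also setting location, energy and material.
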(event OnComponentBeginOverlap(Sphere)
  (params (OverlappedComponent :type Primitive%20Component%20Object%20Reference) (OtherActor :type Actor%20Object%20Reference) (OtherComp :type Primitive%20Component%20Object%20Reference) (OtherBodyIndex :type Integer) (bFromSweep :type Boolean) (SweepResult :type Hit%20Result%20Structure%20%28by%20ref%29))
  (if (and (Utilities|DoesObjectImplementInterface OtherActor "/Game/Blueprints/Player/BPI_Player.BPI_Player_C") (== (Utilities|GetClass OtherComp) "/Script/Engine.SphereComponent"))
    (Variables|Default|SetbPlayerDetected true)
    (Variables|Default|SetPlayerRef OtherActor)
    (Actor|Tick|SetActorTickEnabled true)))

(event EventEnable
  (params (Location :type Vector :default "0, 0, 0") (OrbEnergy :type Float%20%28double-precision%29) (Material :type Material%20Instance%20Object%20Reference))
  (Variables|Default|SetOrbEnergy OrbEnergy)
  (Rendering|Material|SetMaterial (Variables|Default|GetMesh) 0 Material)
  (Actor|Tick|SetActorTickEnabled true)
  (Variables|/Script/Engine.PrimitiveComponent|SetbGenerateOverlapEvents (Variables|Default|GetSphere) true)
  (Collision|SetCollisionEnabled (Variables|Default|GetSphere) "QueryAndPhysics")
  (Rendering|SetActorHiddenInGame false)
  (Transformation|SetActorLocationAndRotation Location "0, 0, 0" false true))

(event EventDisable
  (Actor|Tick|SetActorTickEnabled false)
  (Variables|/Script/Engine.PrimitiveComponent|SetbGenerateOverlapEvents (Variables|Default|GetSphere) false)
  (Collision|SetCollisionEnabled (Variables|Default|GetSphere) "NoCollision")
  (Rendering|SetActorHiddenInGame true))

(event EventBeginPlay
  (Actor|Tick|SetActorTickEnabled false))

(event EventTick
  (params (DeltaSeconds :type Float%20%28single-precision%29))
  (if (Variables|Default|GetbPlayerDetected)
    (Transformation|SetActorLocation (Math|Interpolation|VInterpTo (Transformation|GetActorLocation) (Transformation|GetActorLocation (Variables|Default|GetPlayerRef)) DeltaSeconds 3.0) false false)
    (if (< (Math|Vector2D|Vector2DLength (- (Math|Conversions|ToVector2D(Vector) (Transformation|GetActorLocation (Variables|Default|GetPlayerRef))) (Math|Conversions|ToVector2D(Vector) (Transformation|GetActorLocation)))) 5e+01)
      (Class|BPIPlayer|AddEnergy(Message) (Variables|Default|GetPlayerRef) (Variables|Default|GetOrbEnergy))
      (Default|FreeOrb (Variables|Default|GetOrbManagerRef) self)
      (Variables|Default|SetbPlayerDetected false)
      (Variables|Default|SetPlayerRef 0))))

(fn ConstructionScript)