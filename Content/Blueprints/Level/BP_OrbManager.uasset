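; Orb manager actor that fills the level with energy orbs by day and clears them at night, using an object pool.
; BeginPlay registers placed orbs, pre-spawns pooled ones and binds to GameState day/night events.
; Tick enables or disables one orb per frame until none remain, then switches itself off.
; Spawns use random points in available construction-script boxes and weighted rarity tiers that set energy and material.
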(event Custom|OnDayBegin
  (Actor|Tick|SetActorTickEnabled true)
  (Variables|Default|SetbIsDay true))

(event Custom|OnNightBegin
  (Actor|Tick|SetActorTickEnabled true)
  (Variables|Default|SetbIsDay false))

(event EventBeginPlay
  (bind _gamestate (Class|BPIGameState|GetInstance(Message) (Game|GetGameState)))
  (EventDispatchers|BindEventtoOnDayBeginDispatcher _gamestate (EventDispatchers|CreateEvent :!event Custom|OnDayBegin))
  (EventDispatchers|BindEventtoOnNightBeginDispatcher _gamestate (EventDispatchers|CreateEvent :!event Custom|OnNightBegin))
  (bind _outactors (Actor|GetAllActorsOfClass "/Game/Blueprints/Level/BP_Orb.BP_Orb_C"))
  (for _array_element _outactors
    (Utilities|Map|Add (Variables|Default|GetOrbPool) _array_element true))
  (CallFunction|InitializeOrbPool)
  (CallFunction|OnDayBegin))

(event EventTick
  (params (DeltaSeconds :type Float%20%28single-precision%29))
  (CallFunction|PrintOrbPool)
  (if (Variables|Default|GetbIsDay)
    (bind _spawnlocation (CallFunction|GetSpawnLocation))
    (bind _freeenemy (CallFunction|GetFreeOrb))
    (Utilities|IsValid _freeenemy
      (:Is%20Valid
        (bind _orbtier (CallFunction|GetOrbTier))
        (bind (_orbenergy _material) (CallFunction|SetupOrb _orbtier))
        (Class|BPIOrb|Enable(Message) _freeenemy _spawnlocation _orbenergy _material)
        (Development|PrintString "New Orb Spawned!" false))
      (:Is%20Not%20Valid
        (Development|PrintString "WARNING: No more Orbs in pool!" false)
        (Actor|Tick|SetActorTickEnabled false)))
    (else
      (bind _freeenemy_2 (CallFunction|GetSpawnedOrb))
      (Utilities|IsValid _freeenemy_2
        (:Is%20Valid
          (Class|BPIOrb|Disable(Message) _freeenemy_2)
          (Development|PrintString "Orb Disabled!" false))
        (:Is%20Not%20Valid
          (Development|PrintString "No more orbs to free" false)
          (Actor|Tick|SetActorTickEnabled false))))))

(fn ConstructionScript
  (bind _box (CallFunction|SetupBox (Variables|Positions|GetTopBoxPosition) (Variables|Scale|GetTopBoxScale)))
  (Variables|Default|SetTopBoxRef _box)
  (bind _box_2 (CallFunction|SetupBox (Variables|Positions|GetLeftBoxPosition) (Variables|Scale|GetLeftBoxScale)))
  (Variables|Default|SetLeftBoxRef _box_2)
  (bind _box_3 (CallFunction|SetupBox (Variables|Positions|GetBottomBoxPosition) (Variables|Scale|GetBottomBoxScale)))
  (Variables|Default|SetBottomBoxRef _box_3)
  (bind _box_4 (CallFunction|SetupBox (Variables|Positions|GetRightBoxPosition) (Variables|Scale|GetRightBoxScale)))
  (Variables|Default|SetRightBoxRef _box_4))

(fn InitializeOrbPool
  (for _index (range 1 (Variables|Default|GetOrbPoolSize))
    (bind _returnvalue (Game|SpawnActorfromClass "/Game/Blueprints/Level/BP_Orb.BP_Orb_C" (Math|Transform|MakeTransform "0.000000,0.000000,-500.000000") "AlwaysSpawn" "MultiplyWithRoot" 0 self 0))
    (Utilities|Map|Add (Variables|Default|GetOrbPool) _returnvalue false)))

(fn GetFreeOrb
  (bind _keys (Utilities|Map|Keys (Variables|Default|GetOrbPool)))
  (LocalVariables|Set_OrbPoolKeys _keys)
  (bind _values (Utilities|Map|Values (Variables|Default|GetOrbPool)))
  (if (!= (Utilities|Array|FindItem _values false) -1)
    (Utilities|Map|Add (Variables|Default|GetOrbPool) (Utilities|Array|Get(acopy) (LocalVariables|Get_OrbPoolKeys) (Utilities|Array|FindItem _values false)) true)
    (return (Utilities|Array|Get(acopy) (LocalVariables|Get_OrbPoolKeys) (Utilities|Array|FindItem _values false)))
    (else
      (return 0))))

(fn PrintOrbPool
  (LocalVariables|Set_PoolSize (Utilities|Map|Length (Variables|Default|GetOrbPool)))
  (bind _values (Utilities|Map|Values (Variables|Default|GetOrbPool)))
  (bind _keys (Utilities|Map|Keys (Variables|Default|GetOrbPool)))
  (for (_ _array_index) _keys
    (if (Utilities|Array|Get(acopy) _values _array_index)
      (Math|Integer|IncrementInt (LocalVariables|Get_PoolUsed))
      (else
        (Math|Integer|IncrementInt (LocalVariables|Get_PoolFree)))))
  (Development|PrintString (Utilities|String|ToString(Text) (Utilities|Text|FormatText "Orb Pool Size: {EnemyPoolSize} 
Free: {Free} 
Used: {Used}" (LocalVariables|Get_PoolSize) (LocalVariables|Get_PoolFree) (LocalVariables|Get_PoolUsed))) true false "(R=1.000000,G=0.000000,B=0.000000,A=1.000000)" 2.0 "OrbPool"))

(fn SetupBox
  (params (Position :type Vector) (Scale :type Vector))
  (bind _returnvalue (AddComponent|AddBoxComponent false (Math|Transform|MakeTransform Position)))
  (Components|Box|SetBoxExtent _returnvalue Scale false)
  (Development|SetHiddeninGame _returnvalue false false)
  (Utilities|Map|Add (Variables|Default|GetBoxMap) _returnvalue true)
  (return _returnvalue))

(fn UpdateBox
  (params (OtherActor :type Object%20Object%20Reference) (bMarkAsAvailable :type Boolean) (Box :type Box%20Component%20Object%20Reference))
  (if (Utilities|DoesObjectImplementInterface OtherActor 0)
    (Utilities|Map|Add (Variables|Default|GetBoxMap) Box bMarkAsAvailable)))

(fn GetSpawnLocation
  (bind __availableboxspawns (LocalVariables|Get_AvailableBoxSpawns))
  (bind _outitem (Utilities|Array|Random __availableboxspawns))
  (bind _returnvalue (Transformation|GetWorldLocation _outitem))
  (bind _returnvalue_2 (Components|Box|GetScaledBoxExtent _outitem))
  (bind _returnvalue_3 (Math|Random|RandomPointinBoundingBox _returnvalue _returnvalue_2))
  (bind (_x _y) (Math|Vector|BreakVector _returnvalue_3))
  (bind _keys (Utilities|Map|Keys (Variables|Default|GetBoxMap)))
  (for _array_element _keys
    (if (.Value (Utilities|Map|Find (Variables|Default|GetBoxMap) _array_element))
      (Utilities|Array|Add (LocalVariables|Get_AvailableBoxSpawns) _array_element)))
  (if (Utilities|Array|IsEmpty (LocalVariables|Get_AvailableBoxSpawns))
    (return "0, 0, 0")
    (else
      (return (Math|Vector|MakeVector _x _y 5e+01)))))

(fn DisableAllOrbs)

(fn GetSpawnedOrb
  (bind _keys (Utilities|Map|Keys (Variables|Default|GetOrbPool)))
  (LocalVariables|Set_OrbPoolKeys _keys)
  (bind _values (Utilities|Map|Values (Variables|Default|GetOrbPool)))
  (if (!= (Utilities|Array|FindItem _values true) -1)
    (Utilities|Map|Add (Variables|Default|GetOrbPool) (Utilities|Array|Get(acopy) (LocalVariables|Get_OrbPoolKeys) (Utilities|Array|FindItem _values true)) false)
    (return (Utilities|Array|Get(acopy) (LocalVariables|Get_OrbPoolKeys) (Utilities|Array|FindItem _values true)))
    (else
      (return 0))))

(fn FreeOrb
  (params (Orb :type Actor%20Object%20Reference))
  (Utilities|Map|Add (Variables|Default|GetOrbPool) 0 false)
  (Class|BPIOrb|Disable(Message) Orb))

(fn GetOrbTier
  (LocalVariables|Set_RandomFloat (Math|Random|RandomFloatinRange 0.0 1e+02))
  (for (_array_element _array_index) (Variables|Default|GetRarityWeight)
    (bind _output_get (LocalVariables|Set_CurrentThreshold (+ _array_element (LocalVariables|Get_CurrentThreshold))))
    (if (<= (LocalVariables|Get_RandomFloat) _output_get)
      (return _array_index))))

(fn SetupOrb
  (params (OrbTier :type Integer))
  (switch int OrbTier
    (:0
      (return (Math|Random|RandomFloatinRange 1.5e+03 2.3e+03) "/Game/Materials/M_Orb_Common.M_Orb_Common"))
    (:1
      (return (Math|Random|RandomFloatinRange 2.3e+03 4.2e+03) "/Game/Materials/M_Orb_Uncommon.M_Orb_Uncommon"))
    (:2
      (return (Math|Random|RandomFloatinRange 7e+03 1e+04) "/Game/Materials/M_Orb_Rare.M_Orb_Rare"))
    (:3
      (return (Math|Random|RandomFloatinRange 1.6e+04 2.2e+04) "/Game/Materials/M_Orb_Legendary.M_Orb_Legendary"))))