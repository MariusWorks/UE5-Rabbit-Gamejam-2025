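; Player controller that boots into a menu camera and master widget, then possesses the player pawn when the game state signals game begin.
; While ticking, it turns control rotation toward a cursor ground trace for mouse aiming.
; Game state dispatchers drive begin, end and pause, with Escape toggling pause and input mode.
; It also loads or creates the save object and tallies kills, orbs and damage, though its async save call is unwired.
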(event Custom|OnGamePaused
  (params (GamePaused :type Boolean))
  (if GamePaused
    (Class|WidgetSwitcher|SetActiveWidgetIndex (Variables|/Game/Widgets/WBP_Master.WBP_Master_C|GetWidgetSwitcher (Variables|Default|GetWidget)))
    (Input|SetInputModeUIOnly self (Variables|Default|GetWidget) "DoNotLock" false)
    (else
      (Class|WidgetSwitcher|SetActiveWidgetIndex (Variables|/Game/Widgets/WBP_Master.WBP_Master_C|GetWidgetSwitcher (Variables|Default|GetWidget)) 1)
      (Input|SetInputModeGameOnly self false))))

(event Custom|OnGameBegin
  (Pawn|UnPossess)
  (Transformation|SetActorLocationAndRotation (Variables|Default|GetPawnRef) "0.000000,0.000000,110.000000")
  (Pawn|Possess (Variables|Default|GetPawnRef))
  (Input|AddMappingContext (PlayerController|LocalPlayerSubsystems|GetEnhancedInputLocalPlayerSubsystem self) "/Game/Input/IMC_Default.IMC_Default" 0 "(bIgnoreAllPressedKeysUntilRelease=True,bForceImmediately=False,bNotifyUserSettings=False)")
  (Input|SetInputModeGameOnly self false)
  (Actor|Tick|SetActorTickEnabled true))

(event Custom|OnGameEnd
  (Actor|Tick|SetActorTickEnabled false))

(event EventBeginPlay
  (bind _returnvalue (SaveGame|DoesSaveGameExist "Game"))
  (if _returnvalue
    (bind _returnvalue_2 (SaveGame|LoadGamefromSlot "Game"))
    (bind _asbp_save_game (Utilities|Casting|CastToBP_SaveGame _returnvalue_2)
      (:then
        (Variables|Default|SetSaveGame _asbp_save_game))
      (:CastFailed
        (bind _returnvalue_3 (SaveGame|CreateSaveGameObject "/Game/Blueprints/Game/BP_SaveGame.BP_SaveGame_C" :!label _label))
        (Variables|Default|SetSaveGame _returnvalue_3)))
    (else
      (goto _label)))
  (bind _returnvalue_4 (Actor|GetActorOfClass "/Game/Blueprints/Player/BP_MenuCamera.BP_MenuCamera_C"))
  (Pawn|Possess _returnvalue_4)
  (bind _returnvalue_5 (UserInterface|CreateWidget "/Game/Widgets/WBP_Master.WBP_Master_C" self))
  (bind _output_get (Variables|Default|SetWidget _returnvalue_5))
  (UserInterface|Viewport|AddtoViewport _output_get 0)
  (Input|SetInputModeUIOnly self _output_get "DoNotLock" false)
  (bind _returnvalue_6 (Actor|GetActorOfClass "/Game/Blueprints/Player/BP_PlayerPawn.BP_PlayerPawn_C"))
  (Variables|Default|SetPawnRef _returnvalue_6)
  (bind _gamestate (Class|BPIGameState|GetInstance(Message) (Game|GetGameState)))
  (Variables|Default|SetGameStateRef _gamestate)
  (EventDispatchers|BindEventtoOnGameBeginDispatcher (Variables|Default|GetGameStateRef) (EventDispatchers|CreateEvent :!event Custom|OnGameBegin))
  (EventDispatchers|BindEventtoOnGameEndDispatcher (Variables|Default|GetGameStateRef) (EventDispatchers|CreateEvent :!event Custom|OnGameEnd))
  (EventDispatchers|BindEventtoOnGamePausedDispatcher (Variables|Default|GetGameStateRef) (EventDispatchers|CreateEvent :!event Custom|OnGamePaused)))

(event EventTick
  (params (DeltaSeconds :type Float%20%28single-precision%29))
  (bind (_bouthit _hitlocation) (CallFunction|TraceforGround))
  (if _bouthit
    (Pawn|SetControlRotation (Math|Rotator|FindLookatRotation (Transformation|GetActorLocation (Pawn|GetControlledPawn)) _hitlocation))))

(event EventAddKill
  (params (EnemyName :type Name :default "None"))
  (bind _playerscore (Variables|Default|GetPlayerScore))
  (bind _kills (Utilities|Struct|BreakS_PlayerScore _playerscore))
  (bind (_value _returnvalue) (Utilities|Map|Find _kills EnemyName))
  (if _returnvalue
    (Utilities|Map|Add _kills EnemyName (+ _value 1))
    (else
      (Utilities|Map|Add _kills EnemyName 1))))

(event EventAddOrb
  (params (OrbName :type Name :default "None"))
  (bind _playerscore (Variables|Default|GetPlayerScore))
  (bind _orbscollected (Utilities|Struct|BreakS_PlayerScore _playerscore))
  (bind (_value _returnvalue) (Utilities|Map|Find _orbscollected OrbName))
  (if _returnvalue
    (Utilities|Map|Add _orbscollected OrbName (+ _value 1))
    (else
      (Utilities|Map|Add _orbscollected OrbName 1))))

(event EventAddDamageTaken
  (params (Damage :type Float%20%28double-precision%29))
  (bind _playerscore (Variables|Default|GetPlayerScore))
  (bind _damagetaken (Utilities|Struct|BreakS_PlayerScore _playerscore))
  (|SetBy-RefVar _damagetaken (+ Damage _damagetaken)))

(event EventAddDamageDealt
  (params (Damage :type Float%20%28double-precision%29))
  (bind _playerscore (Variables|Default|GetPlayerScore))
  (bind _damagedone (Utilities|Struct|BreakS_PlayerScore _playerscore))
  (|SetBy-RefVar _damagedone (+ Damage _damagedone)))

(event Input|KeyboardEvents|Escape
  (params (Key :type Key%20Structure :default "None"))
  (:Pressed
    (if (Variables|/Game/Blueprints/Game/BP_GameState.BP_GameState_C|GetbGameIsPaused (Variables|Default|GetGameStateRef))
      (Default|CallOnGamePausedDispatcher (Variables|Default|GetGameStateRef) false)
      (else
        (Default|CallOnGamePausedDispatcher (Variables|Default|GetGameStateRef) true) ; This should never fire but I have trust issues
      ))))

(fn ConstructionScript)

(fn TraceforGround
  (bind (_locationx _locationy) (Game|Player|GetMousePosition))
  (bind _self self)
  (bind _returnvalue (Math|Vector2D|MakeVector2D _locationx _locationy))
  (bind (_worldposition _worlddirection) (Class|GameplayStatics|DeprojectScreentoWorld _self _returnvalue))
  (bind (_outhit _returnvalue_2) (Collision|LineTraceForObjects _worldposition (+ _worldposition (* _worlddirection 1e+06)) (Utilities|Array|MakeArray "ObjectTypeQuery1") false 0 "None"))
  (if _returnvalue_2
    (return true (.Location (Collision|BreakHitResult _outhit)))
    (else
      (return false "0, 0, 0"))))

(fn PrintPlayerScore
  (bind _playerscore (Variables|Default|GetPlayerScore))
  (bind (_kills _orbscollected _damagedone _damagetaken) (Utilities|Struct|BreakS_PlayerScore _playerscore))
  (bind _keys (Utilities|Map|Keys _kills))
  (for _array_element _keys
    (LocalVariables|Set_KillsString (Utilities|String|Append (LocalVariables|Get_KillsString) (Utilities|String|ToString(Text) (Utilities|Text|FormatText " 
{Kills} {EnemyName} Kills " (.Value (Utilities|Map|Find _kills _array_element)) _array_element)))))
  (Development|PrintString (Utilities|String|ToString(Text) (Utilities|Text|FormatText "PlayerScore: 
{Kills} 
Orbs Collected: {OrbsCollected} 
Damage Done: {DamageDone} 
Damage Taken: {DamageTaken}" (LocalVariables|Get_KillsString) 0 _damagedone _damagetaken)) true false "(R=0.128853,G=0.618748,B=1.000000,A=1.000000)" 0.0 "PlayerScore"))

(fn GetPlayerLastRunScore
  (Utilities|IsValid (Variables|Default|GetSaveGame)
    (:Is%20Valid
      (return (Variables|/Game/Blueprints/Game/BP_SaveGame.BP_SaveGame_C|GetPlayerLastRunScore (Variables|Default|GetSaveGame))))
    (:Is%20Not%20Valid
      (return (Variables|Default|GetPlayerScoreLastRun)))))

(fn GetPlayerTotalScore
  (Utilities|IsValid (Variables|Default|GetSaveGame)
    (:Is%20Valid
      (return (Variables|/Game/Blueprints/Game/BP_SaveGame.BP_SaveGame_C|GetPlayerScore (Variables|Default|GetSaveGame))))
    (:Is%20Not%20Valid
      (return (Variables|Default|GetPlayerScore)))))