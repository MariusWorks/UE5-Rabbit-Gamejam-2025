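; Player pawn with movement, sprint, dodge and sword-and-shield melee combat, driven by Enhanced Input and a PlayerStats struct.
; Timelines animate attack, block, dodge, knockback and shield nudge, moving the pawn by swept world offsets.
; Mid-swing, a box trace sends damage to BPI_Enemy actors.
; Sprinting and shield hits drain stamina, which gates sprint and dodge through exhaustion checks, while Tick recharges it, counts down dodge cooldown and prints stats.
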(event Input|EnhancedActionEvents|EnhancedInputActionIA_Attack
  (params (ActionValue :type Boolean) (ElapsedSeconds :type Float%20%28double-precision%29) (TriggeredSeconds :type Float%20%28double-precision%29) (InputAction :type Input%20Action%20Object%20Reference :default "/Game/Input/Actions/IA_Attack.IA_Attack"))
  (:Started
    (if (not (Math|Boolean|ORBoolean (Variables|Default|GetbSprinting) (Variables|Default|GetbDodging) (Variables|Default|GetbIsBlocking) (Variables|Default|GetbAttacking)))
      (Variables|Default|SetbAttacking true)
      (Components|Timeline|SetPlayRate (Variables|Default|GetTimeline_Attack) (/ 1.0 (Math|Float|MakeLiteralFloat 0.1)))
      (bind _alpha (Timeline|Timeline_Attack PlayFromStart)
        (:Update
          (Transformation|SetRelativeTransform (Variables|Default|GetSword) (Math|Transform|Lerp(Transform) (Variables|SwordAnimation|GetDefaultSwordTransform) (Variables|SwordAnimation|GetTargetSwordTransform) _alpha) false false)
          (if (> _alpha 0.5)
            (Utilities|FlowControl|DoOnce false :!label _label
              (:Completed
                (bind _hitactors (CallFunction|AttackGetOverlappingActors))
                (for _array_element _hitactors
                  (Class|BPICombat|OnDamage(Message) _array_element (.Damage (Utilities|Struct|BreakS_PlayerStats (Variables|Default|GetPlayerStats))) self))))))
        (:Finished
          (Variables|Default|SetbAttacking false)
          (Transformation|SetRelativeTransform (Variables|Default|GetSword) (Variables|SwordAnimation|GetDefaultSwordTransform) false false)
          (goto _label Reset))))))

(event Input|EnhancedActionEvents|EnhancedInputActionIA_Block
  (params (ActionValue :type Boolean) (ElapsedSeconds :type Float%20%28double-precision%29) (TriggeredSeconds :type Float%20%28double-precision%29) (InputAction :type Input%20Action%20Object%20Reference :default "/Game/Input/Actions/IA_Block.IA_Block"))
  (:Started
    (Collision|SetCollisionEnabled (Variables|Default|GetShieldBox) "QueryOnly")
    (Variables|Default|SetbIsBlocking true)
    (Components|Timeline|SetPlayRate (Variables|Default|GetTimeline_Block) (/ 1.0 (Math|Float|MakeLiteralFloat 0.1)))
    (bind _alpha (Timeline|Timeline_Block PlayFromStart)
      (:Update
        (Transformation|SetRelativeTransform (Variables|Default|GetShield) (Math|Transform|Lerp(Transform) (Variables|ShieldAnimation|GetDefaultShieldTransform) (Variables|ShieldAnimation|GetTargetShieldTransform) _alpha) false false))
      (:Finished
        (if (Variables|Default|GetbIsBlocking)
          (Transformation|SetRelativeTransform (Variables|Default|GetShield) (Variables|ShieldAnimation|GetTargetShieldTransform) false false)
          (else
            (Transformation|SetRelativeTransform (Variables|Default|GetShield) (Variables|ShieldAnimation|GetDefaultShieldTransform) false false))))))
  (:Completed
    (Collision|SetCollisionEnabled (Variables|Default|GetShieldBox) "NoCollision")
    (Variables|Default|SetbIsBlocking false)
    (Timeline|Timeline_Block Reverse)))

(event Input|EnhancedActionEvents|EnhancedInputActionIA_Sprint
  (params (ActionValue :type Boolean) (ElapsedSeconds :type Float%20%28double-precision%29) (TriggeredSeconds :type Float%20%28double-precision%29) (InputAction :type Input%20Action%20Object%20Reference :default "/Game/Input/Actions/IA_Sprint.IA_Sprint"))
  (:Triggered
    (if (CallFunction|CanPlayerSprint)
      (CallFunction|SetPlayerSprinting true)
      (CallFunction|DrainStamina)
      (else
        (CallFunction|CheckPlayerExhausted :!label _label)
        (CallFunction|SetPlayerSprinting false))))
  (:Completed
    (goto _label)))

(event Input|EnhancedActionEvents|EnhancedInputActionIA_Dodge
  (params (ActionValue :type Boolean) (ElapsedSeconds :type Float%20%28double-precision%29) (TriggeredSeconds :type Float%20%28double-precision%29) (InputAction :type Input%20Action%20Object%20Reference :default "/Game/Input/Actions/IA_Dodge.IA_Dodge"))
  (bind _playerstats (Variables|Default|GetPlayerStats))
  (bind (_health _maxstamina _stamina _speed _sprintspeed _damage _defense _staminadrainrate _staminarechargerate _exhaustedthreshold _dodgecooldown _dodgeduration) (Utilities|Struct|BreakS_PlayerStats _playerstats))
  (if (CallFunction|CanPlayerDodge)
    (Variables|Default|SetbDodging true)
    (Variables|Default|SetDodgeCooldown _dodgecooldown)
    (Components|Timeline|SetPlayRate (Variables|Default|GetTimeline_Dodge) (/ 1.0 _dodgeduration))
    (Variables|Default|SetMoveActionValue (Input|EnhancedActionValues|GetIA_Move))
    (Timeline|Timeline_Dodge PlayFromStart
      (:Update
        (Transformation|AddActorWorldOffset (* (CallFunction|NormalizeActionValue (Variables|Default|GetMoveActionValue)) (* (.DodgeSpeed (Utilities|Struct|BreakS_PlayerStats (Variables|Default|GetPlayerStats))) (Utilities|Time|GetWorldDeltaSeconds))) true))
      (:Finished
        (Variables|Default|SetbDodging false)))))

(event Input|EnhancedActionEvents|EnhancedInputActionIA_Move
  (params (ActionValue :type Vector%202D%20Structure) (ElapsedSeconds :type Float%20%28double-precision%29) (TriggeredSeconds :type Float%20%28double-precision%29) (InputAction :type Input%20Action%20Object%20Reference :default "/Game/Input/Actions/IA_Move.IA_Move"))
  (if (CallFunction|CanPlayerMove)
    (Transformation|AddActorWorldOffset (* (CallFunction|NormalizeActionValue ActionValue) (* (Variables|Default|GetPlayerSpeed) (Utilities|Time|GetWorldDeltaSeconds))) true)))

(event EventBeginPlay)

(event EventOnDamage
  (params (Damage :type Float%20%28double-precision%29) (Attacker :type Actor%20Object%20Reference))
  (bind _playerstats (Variables|Default|GetPlayerStats))
  (bind _health (Utilities|Struct|BreakS_PlayerStats _playerstats))
  (bind _returnvalue (- _health Damage))
  (bind _returnvalue_2 (<= _returnvalue 0.0))
  (|SetBy-RefVar _health (select _returnvalue_2 0.0 _returnvalue))
  (if (not _returnvalue_2)
    (Variables|Default|SetKnockbackDirection (Math|Vector|Normalize (- (Transformation|GetActorLocation) (Transformation|GetActorLocation Attacker))))
    (Timeline|Timeline_Knockback PlayFromStart
      (:Update
        (Transformation|AddActorWorldOffset (* (Variables|Default|GetKnockbackDirection) (* 5e+02 (Utilities|Time|GetWorldDeltaSeconds))) true)))))

(event EventOnShield
  (bind _playerstats (Variables|Default|GetPlayerStats))
  (bind (_health _maxstamina _stamina _speed _sprintspeed _damage _defense _staminadrainrate _staminarechargerate _exhaustedthreshold _dodgecooldown _dodgeduration _dodgespeed _dodgecost _blockcost) (Utilities|Struct|BreakS_PlayerStats _playerstats))
  (|SetBy-RefVar _stamina (- _stamina _blockcost))
  (bind _alpha (Timeline|Timeline_ShieldNudge PlayFromStart)
    (:Update
      (Transformation|SetRelativeRotation (Variables|Default|GetShield) (Math|Rotator|MakeRotator (* _alpha 2e+01) 0.0 0.0) false false))))

(event EventTick
  (params (DeltaSeconds :type Float%20%28single-precision%29))
  (CallFunction|PrintPlayerStats)
  (CallFunction|RechargeStamina)
  (CallFunction|RechargeDodge))

(fn ConstructionScript)

(fn NormalizeActionValue
  (params (ActionValue :type Vector%202D%20Structure))
  (bind (_x _y) (Math|Vector2D|BreakVector2D ActionValue))
  (return (Math|Vector|ClampVectorSize (+ (* "0.000000,1.000000,0.000000" _x) (* "1.000000,0.000000,0.000000" _y)) 0.0 1.0)))

(fn PrintPlayerStats
  (bind _playerstats (Variables|Default|GetPlayerStats))
  (Development|PrintString (Utilities|String|ToString(Text) (Utilities|Text|FormatText "Player Stats: 
Health: {Health} 
Stamina: {Stamina} 
Speed: {Speed} 
Damage: {Damage} 
Defense: {Defense}" (.health _playerstats) (.stamina _playerstats) (.speed _playerstats) (.damage _playerstats) (.defense _playerstats))) true false "(R=0.000000,G=1.000000,B=0.000000,A=1.000000)" 0.0 "PlayerStats"))

(fn CanPlayerSprint
  (return (and (> (.stamina (Variables|Default|GetPlayerStats)) 0.0) (not (Variables|Default|GetbExhausted)))))

(fn DrainStamina
  (bind _returnvalue (Utilities|Time|GetWorldDeltaSeconds))
  (bind _playerstats (Variables|Default|GetPlayerStats))
  (bind _returnvalue_2 (* (.staminadrainrate _playerstats) _returnvalue))
  (bind _returnvalue_3 (- (.stamina _playerstats) _returnvalue_2))
  (|SetBy-RefVar (.stamina _playerstats) (Math|Float|SelectFloat 0.0 _returnvalue_3 (< _returnvalue_3 0.0))))

(fn RechargeStamina
  (bind _returnvalue (Utilities|Time|GetWorldDeltaSeconds))
  (bind _playerstats (Variables|Default|GetPlayerStats))
  (bind (_health _maxstamina _stamina _speed _sprintspeed _damage _defense _staminadrainrate) (Utilities|Struct|BreakS_PlayerStats _playerstats))
  (bind _returnvalue_2 (* _staminadrainrate _returnvalue))
  (bind _returnvalue_3 (+ _stamina _returnvalue_2))
  (bind _returnvalue_4 (> _returnvalue_3 _maxstamina))
  (bind _returnvalue_5 (Math|Float|SelectFloat _maxstamina _returnvalue_3 _returnvalue_4))
  (if (not (or (Variables|Default|GetbSprinting) (Variables|Default|GetbIsBlocking)))
    (|SetBy-RefVar _stamina _returnvalue_5)
    (if (> _returnvalue_5 (.ExhaustedThreshold (Utilities|Struct|BreakS_PlayerStats (Variables|Default|GetPlayerStats))))
      (Variables|Default|SetbExhausted false))))

(fn SetPlayerSprinting
  (params (bPlayerSprinting :type Boolean))
  (bind _playerstats (Variables|Default|GetPlayerStats))
  (bind (_health _maxstamina _stamina _speed _sprintspeed) (Utilities|Struct|BreakS_PlayerStats _playerstats))
  (bind _output_get (Variables|Default|SetbSprinting bPlayerSprinting))
  (Variables|Default|SetPlayerSpeed (select _output_get _sprintspeed _speed)))

(fn CheckPlayerExhausted
  (bind _playerstats (Variables|Default|GetPlayerStats))
  (bind (_health _maxstamina _stamina _speed _sprintspeed _damage _defense _staminadrainrate _staminarechargerate _exhaustedthreshold) (Utilities|Struct|BreakS_PlayerStats _playerstats))
  (Variables|Default|SetbExhausted (< _stamina _exhaustedthreshold)))

(fn CanPlayerDodge
  (bind _playerstats (Variables|Default|GetPlayerStats))
  (return (Math|Boolean|ANDBoolean (> (.stamina _playerstats) 0.0) (not (Variables|Default|GetbExhausted)) (not (Variables|Default|GetbDodging)) (> (.stamina _playerstats) (.dodgecost _playerstats)) (<= (Variables|Default|GetDodgeCooldown) 0.0))))

(fn CanPlayerMove
  (if (Variables|Default|GetbDodging)
    (return false)
    (else
      (return true))))

(fn RechargeDodge
  (Variables|Default|SetDodgeCooldown (select (<= (- (Variables|Default|GetDodgeCooldown) (Utilities|Time|GetWorldDeltaSeconds)) 0.0) 0.0 (- (Variables|Default|GetDodgeCooldown) (Utilities|Time|GetWorldDeltaSeconds)))))

(fn AttackGetOverlappingActors
  (bind _swordbox (Variables|Default|GetSwordBox))
  (bind _returnvalue (Transformation|GetWorldLocation _swordbox))
  (bind (_outhits _returnvalue_2) (Class|KismetSystemLibrary|BoxTraceMultiforObjects _returnvalue _returnvalue (Components|Box|GetScaledBoxExtent (Variables|Default|GetSwordBox)) (Transformation|GetWorldRotation (Variables|Default|GetSwordBox)) (Utilities|Array|MakeArray "ObjectTypeQuery3") false (Utilities|Array|MakeArray self) "None" true))
  (if _returnvalue_2
    (for _array_element _outhits
      (if (Utilities|DoesObjectImplementInterface (.HitActor (Collision|BreakHitResult _array_element)) "/Game/Blueprints/Enemy/BPI_Enemy.BPI_Enemy_C")
        (Utilities|Array|Add (LocalVariables|Get_HitEnemies) (.HitActor (Collision|BreakHitResult _array_element)))))
    (return (LocalVariables|Get_HitEnemies))))

(fn GetCanBlock
  (bind _playerstats (Variables|Default|GetPlayerStats))
  (bind (_health _maxstamina _stamina _speed _sprintspeed _damage _defense _staminadrainrate _staminarechargerate _exhaustedthreshold _dodgecooldown _dodgeduration _dodgespeed _dodgecost _blockcost) (Utilities|Struct|BreakS_PlayerStats _playerstats))
  (return (>= _stamina _blockcost)))

(fn GetPlayerShields
  (return 0))